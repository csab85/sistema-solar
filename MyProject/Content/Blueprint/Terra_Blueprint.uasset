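; Terra Blueprint is a planet actor that spins on its yaw axis and is set up to orbit a sun at the world origin.
; BeginPlay stores its distance from the origin as SunDistance.
; Each Tick rotates it, adds a cosine/sine offset of that radius to its current location rather than the origin, flattens Z, and prints Angle.
; IncreaseAngle is unconnected, so Angle never advances and the offset direction stays fixed.
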(event EventBeginPlay
  (|GetSunDistance))

(event Collision|EventActorBeginOverlap
  (params (OtherActor :type Actor%20Object%20Reference)))

(event EventTick
  (params (DeltaSeconds :type Float%20%28single-precision%29))
  (bind _returnvalue (Transformation|GetActorLocation))
  (bind (_x _y) (Math|Vector|BreakVector _returnvalue))
  (Utilities|FlowControl|Sequence
    (:then_0
      (|Rotation DeltaSeconds))
    (:then_2
      (Transformation|SetActorLocation (Math|Vector|MakeVector (+ _x (* (Math|Trig|Cos(Radians) (Variables|Default|Getangle)) (Variables|Default|GetsunDistance))) (+ _y (* (Math|Trig|Sin(Radians) (Variables|Default|Getangle)) (Variables|Default|GetsunDistance))) 0.0) false false))
    (:then_3
      (Development|PrintText (Utilities|Text|ToText(Float) (Variables|Default|Getangle) "HalfToEven")))))

(fn ConstructionScript)