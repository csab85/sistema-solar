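; Mars (Marte) planet actor that spins on its axis and orbits the world origin, treated as the Sun's position.
; On BeginPlay it stores its distance from the origin as the orbit radius.
; Each Tick it applies a delta-time scaled local yaw, advances the orbit angle by the translation speed, then sets X and Y from sine and cosine of that angle for a circular path.
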(event EventBeginPlay
  (|SetSunDistance))

(event EventTick
  (params (DeltaSeconds :type Float%20%28single-precision%29))
  (Utilities|FlowControl|Sequence
    (:then_0
      (|Rotation DeltaSeconds))
    (:then_1
      (|IncreaseAngle DeltaSeconds)
      (|UpdatePosition))))

(fn ConstructionScript)